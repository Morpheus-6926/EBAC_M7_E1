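; BP_Stone is a pickup actor that pulses in size and explodes when collected.
; A Delay-driven loop from BeginPlay samples a float curve with a wrapping timer to scale the actor above its base size, without using Tick or a Timeline.
; On overlap with an actor implementing BPI_Interactions, it sends PickUpMessage, destroys itself, and plays an explosion particle and 2D sound.
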(event `self.ReceiveBeginPlay`
  (`self.SetActorScale3D` (+ (* (0.5 0.5 0.5) (`CurveFloat.GetFloatValue` (`self.Curve`) (`self.TimerPulse`))) (1.0 1.0 1.0)) :!label _label)
  (set `self.TimerPulse` (+ (`self.TimerPulse`) 0.01))
  (if (> (`self.TimerPulse`) 1.0)
    (set `self.TimerPulse` 0.0))
  (`KismetSystemLibrary.Delay` 0.01)
  (goto _label))

(event `self.ReceiveActorBeginOverlap`
  (params (OtherActor :type "Actor Object Reference"))
  (if (`KismetSystemLibrary.DoesImplementInterface` OtherActor "/Game/EBAC/Blueprints/BPI_Interactions.BPI_Interactions_C")
    (message `/Game/EBAC/Blueprints/BPI_Interactions.PickUp` OtherActor)
    (`self.K2_DestroyActor`)
    (`GameplayStatics.SpawnEmitterAtLocation` "/Game/StarterContent/Particles/P_Explosion.P_Explosion" (`self.K2_GetActorLocation`))
    (`GameplayStatics.PlaySound2D` "/Game/StarterContent/Audio/Explosion01.Explosion01" 1.0 1.0 0.0 null null)))

(fn `UserConstructionScript`)