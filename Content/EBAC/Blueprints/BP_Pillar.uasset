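; BP_Pillar is a pillar actor that moves vertically in a repeating, curve-driven cycle.
; It caches its start location at construction; after a delay, StartMove loops on short timed delays, offsetting Z by MoveCurve scaled by MoveDistance.
; Curve time advances by TimeScale steps and wraps after passing one.
; Lower stops the cycle and sets relative Z to a fixed height, retrying while world Z is below zero.
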(event `StartMove`
  (bind (_initlocation_x _initlocation_y) (`KismetMathLibrary.BreakVector` (`self.InitLocation`)))
  (`KismetSystemLibrary.Delay` (`self.DelayToStart`))
  (if (`self.Move`) :!label _label
    (`self.K2_SetActorRelativeLocation` (+ (0.0 0.0 0.0) (`KismetMathLibrary.MakeVector` _initlocation_x _initlocation_y (+ 0.0 (* (`CurveFloat.GetFloatValue` (`self.MoveCurve`) (`self.InTime`)) (`self.MoveDistance`))))))
    (bind _output_get (set `self.InTime` (+ (`self.InTime`) (* (`self.TimeScale`) 0.001))))
    (if (> _output_get 1.0)
      (set `self.InTime` 0.0)))
  (`KismetSystemLibrary.Delay` (* (`self.TimeScale`) 0.001))
  (goto _label))

(event `Lower`
  (bind (_returnvalue_x _returnvalue_y _returnvalue_z) (`KismetMathLibrary.BreakVector` (`self.K2_GetActorLocation`)))
  (bind (_initlocation_x _initlocation_y) (`KismetMathLibrary.BreakVector` (`self.InitLocation`)))
  (set `self.Move` false)
  (`self.K2_SetActorRelativeLocation` (`KismetMathLibrary.MakeVector` _initlocation_x _initlocation_y 100.0) :!label _label_2)
  (if (> 0.0 _returnvalue_z)
    (`KismetSystemLibrary.Delay` 0.1)
    (goto _label_2)))

(fn `UserConstructionScript`
  (set `self.InitLocation` (`self.K2_GetActorLocation`)))